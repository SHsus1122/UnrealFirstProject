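; BP_Sphere_Child_Moving is a child sphere Blueprint that bobs its Sphere component up and down continuously.
; Each Tick it adds a relative Z offset, using the IsLoopingEnd flag for direction and flipping it when world Z reaches UpLocation or DownLocation.
; The step adds DeltaSeconds to positive or negative Speed instead of multiplying, so movement depends on frame rate.
; The construction script calls the parent's; the overlap override is disabled.
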(event EventBeginPlay)

(event Collision|EventActorBeginOverlap
  (params (OtherActor :type Actor%20Object%20Reference))
  (|CallParentFunction OtherActor) ; 지금 이 노드는 비활성 상태입니다. \n핀을 끌어서 다른 노드를 연결하면 활성화됩니다.
)

(event EventTick
  (params (DeltaSeconds :type Float%20%28single-precision%29))
  (bind _sphere (Variables|Default|GetSphere))
  (bind _sphere_2 (Variables|Default|GetSphere))
  (if (Variables|Default|GetIsLoopingEnd)
    (Transformation|AddRelativeLocation _sphere_2 (Math|Vector|MakeVector 0.0 0.0 (+ (Variables|Default|GetSpeed) DeltaSeconds)) false false)
    (if (>= (.z (Transformation|GetWorldLocation _sphere_2)) (Variables|Default|GetUpLocation))
      (Variables|Default|SetIsLoopingEnd false))
    (else
      (Transformation|AddRelativeLocation _sphere (Math|Vector|MakeVector 0.0 0.0 (- DeltaSeconds (Variables|Default|GetSpeed))) false false)
      (if (<= (.z (Transformation|GetWorldLocation _sphere)) (Variables|Default|GetDownLocation))
        (Variables|Default|SetIsLoopingEnd true)))))

(fn ConstructionScript
  (|CallParentFunction))