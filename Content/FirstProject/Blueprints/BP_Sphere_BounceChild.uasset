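; Child Blueprint of a sphere actor that makes the sphere keep bouncing whenever it drops low.
; Each Tick runs the parent logic, then checks GCSphere's height against a fixed world Z threshold.
; While it is below, Sphere receives a randomized, mass-independent velocity impulse, mostly upward with slight positive X/Y drift, with no cooldown between frames.
; BeginPlay and overlap events are disabled placeholders, and construction only calls the parent.
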(event EventBeginPlay
  (|CallParentFunction) ; 지금 이 노드는 비활성 상태입니다. \n핀을 끌어서 다른 노드를 연결하면 활성화됩니다.
)

(event Collision|EventActorBeginOverlap
  (params (OtherActor :type Actor%20Object%20Reference))
  (|CallParentFunction OtherActor) ; 지금 이 노드는 비활성 상태입니다. \n핀을 끌어서 다른 노드를 연결하면 활성화됩니다.
)

(event EventTick
  (params (DeltaSeconds :type Float%20%28single-precision%29))
  (|CallParentFunction DeltaSeconds)
  (if (< (.z (Transformation|GetSocketLocation (Variables|Default|GetGC_Sphere) "None")) 1e+02)
    (Physics|AddImpulse (Variables|Default|GetSphere) (Math|Vector|MakeVector (Math|Random|RandomFloatinRange 1e+01 45.0) (Math|Random|RandomFloatinRange 1e+01 45.0) (Math|Random|RandomFloatinRange 1e+03 1.2e+03)) "None" true)))

(fn ConstructionScript
  (|CallParentFunction))