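; BP_Rock1 is a damageable rock actor that is launched shortly after spawning, then falls.
; BeginPlay applies a velocity-change impulse to its Capsule, then enables gravity after a delay.
; A hit while gravity is on freezes the Capsule, reattaches GCRock to Scene and hands physics and collision over to it.
; Each damage event subtracts one HP regardless of amount, destroying the actor below zero.
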(event OnComponentHit(Capsule)
  (params (HitComponent :type Primitive%20Component%20Object%20Reference) (OtherActor :type Actor%20Object%20Reference) (OtherComp :type Primitive%20Component%20Object%20Reference) (NormalImpulse :type Vector :default "0, 0, 0") (Hit :type Hit%20Result%20Structure%20%28by%20ref%29))
  (bind _capsule (Variables|Default|GetCapsule))
  (bind _gc_rock (Variables|Default|GetGC_Rock))
  (if (Class|PrimitiveComponent|IsGravityEnabled _capsule)
    (Physics|SetEnableGravity _capsule false)
    (Physics|SetSimulatePhysics _capsule false)
    (Transformation|AttachComponentToComponent (Variables|Default|GetGC_Rock) (Variables|Default|GetScene) "None" "KeepWorld" "KeepWorld" "KeepWorld" true)
    (Utilities|FlowControl|Delay 0.1)
    (Collision|SetCollisionEnabled _capsule "NoCollision")
    (Physics|SetSimulatePhysics _gc_rock true)
    (Collision|SetCollisionEnabled _gc_rock "QueryAndPhysics")))

(event Custom|OnDestory)

(event EventBeginPlay
  (Utilities|FlowControl|Delay 0.2)
  (Physics|AddImpulse (Variables|Default|GetCapsule) "0.000000,50.000000,100.000000" "None" true)
  (Utilities|FlowControl|Delay 2.0)
  (Physics|SetEnableGravity (Variables|Default|GetCapsule) true))

(event Collision|EventActorBeginOverlap
  (params (OtherActor :type Actor%20Object%20Reference)))

(event EventTick
  (params (DeltaSeconds :type Float%20%28single-precision%29)))

(event Game|Damage|EventAnyDamage
  (params (Damage :type Float%20%28single-precision%29) (DamageType :type Damage%20Type%20Object%20Reference) (InstigatedBy :type Controller%20Object%20Reference) (DamageCauser :type Actor%20Object%20Reference))
  (bind _result (Math|Float|DecrementFloat (Variables|컴포넌트|GetHP))
    (:%20%20
      (bind _output_get (Variables|컴포넌트|SetHP _result))
      (Development|PrintString (Utilities|String|ToString(Float) _output_get))
      (if (< _output_get 0.0)
        (Actor|DestroyActor)
        (Development|PrintString "사망")))))

(fn ConstructionScript)